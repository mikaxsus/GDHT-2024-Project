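; Collider ball actor that makes foliage react to its presence.
; Each Tick it writes its location to the BallPos parameter in MPC_Master, sharing it with materials.
; It also runs a zero-length multi sphere trace on Visibility using its Sphere radius, sending each hit component a WobbleMessage with item index and location.
; An author note recommends a custom trace channel for wobble foliage to improve performance.
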(event EventTick
  (params (DeltaSeconds :type Float%20%28single-precision%29))
  (bind _returnvalue (Transformation|GetActorLocation))
  (Rendering|Material|SetVectorParameterValue "/Game/Assets/StylizedShaders/Materials/MaterialParameterCollection/MPC_Master.MPC_Master" "BallPos" (Math|Conversions|ToLinearColor(Vector) (Transformation|GetActorLocation)) :!class /Script/Engine.KismetMaterialLibrary)
  (bind (_outhits _returnvalue_2) (Collision|MultiSphereTraceByChannel _returnvalue _returnvalue (Components|Sphere|GetScaledSphereRadius (Variables|Default|GetSphere)) "TraceTypeQuery1" false 0 "None")) ; Ideally, you want to set up a custom trace channel for\nyour wobble foliage to optimize performance.
  (if _returnvalue_2
    (for _array_element _outhits
      (Class|BPIFoliageWobbleNew|Wobble(Message) (.HitComponent (Collision|BreakHitResult _array_element)) (.HitItem (Collision|BreakHitResult _array_element)) (.Location (Collision|BreakHitResult _array_element))))))

(fn ConstructionScript)