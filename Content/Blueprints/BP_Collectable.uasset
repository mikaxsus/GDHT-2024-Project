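; Coin pickup for a four-player car game that credits the collecting car's player and announces the winner.
; On overlap with a VehicleAdvPawn, it matches the TeamColor name by substring to a player index.
; It increments that BPC_CarGame controller's coin count and destroys itself.
; When the count hits three, it creates a W_Winner widget owned by the first player, showing the winning player's text.
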(event OnComponentBeginOverlap(Collision)
  (params (OverlappedComponent :type Primitive%20Component%20Object%20Reference) (OtherActor :type Actor%20Object%20Reference) (OtherComp :type Primitive%20Component%20Object%20Reference) (OtherBodyIndex :type Integer) (bFromSweep :type Boolean) (SweepResult :type Hit%20Result%20Structure%20%28by%20ref%29))
  (bind _asvehicle_adv_pawn (Utilities|Casting|CastToVehicleAdvPawn OtherActor))
  (bind _output_get (Variables|Default|SetsCollector (Utilities|String|ToString(Object) (Variables|/Game/Blueprints/Vehicles/Default/VehicleAdvPawn.VehicleAdvPawn_C|GetTeamColor _asvehicle_adv_pawn))))
  (Utilities|WhoCollectedMe? _output_get)
  (bind _asbpc_car_game (Utilities|Casting|CastToBPC_CarGame (Game|GetPlayerController (Variables|Default|GetiWhoCollected))))
  (bind _result (Math|Integer|IncrementInt (Variables|/Game/Blueprints/Input/Controllers/BPC_CarGame.BPC_CarGame_C|GetiCoins _asbpc_car_game))
    (:%20%20
      (Actor|DestroyActor)
      (if (== _result 3)
        (Utilities|WhoWon? (Variables|Default|GetsCollector))
        (bind _returnvalue (UserInterface|CreateWidget "/Game/UI/W_Winner.W_Winner_C" (Game|GetPlayerController 0)))
        (Variables|/Game/UI/W_Winner.W_Winner_C|SetWinnerText _returnvalue (Variables|Default|GettWhoWonThisGame))
        (UserInterface|Viewport|AddtoViewport _returnvalue 0)))))

(fn ConstructionScript)